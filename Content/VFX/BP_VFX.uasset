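; BP_VFX is an effect actor that plays a turbo effect with an animated point light once on BeginPlay.
; It zeroes the light, then starts three timelines from a sequence.
; Two timelines animate only the Z of the NSTurbo Scale and Scale2 vector parameters over fixed XY, and the third drives light intensity.
; A delayed replay branch exists but is disconnected, so it never runs.
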(event `self.ReceiveBeginPlay`
  (`LightComponent.SetIntensity` (`self.PointLight`) 0.0)
  (`|ExecutionSequence`
    (:`then_0`
      (bind (_direction _scalez) (`Timeline|TimeFX_Start` :!via `PlayFromStart`)
        (:`Update`
          (`FXSystemComponent.SetVectorParameter` (`self.NS_Turbo`) "Scale" (`KismetMathLibrary.MakeVector` 14.0 14.0 _scalez)))))
    (:`then_1`
      (bind (_direction_2 _scalez_2) (`Timeline|TimeFX` :!via `PlayFromStart`)
        (:`Update`
          (`FXSystemComponent.SetVectorParameter` (`self.NS_Turbo`) "Scale2" (`KismetMathLibrary.MakeVector` 8.0 8.0 _scalez_2)))))
    (:`then_2`
      (bind (_direction_3 _intensitylight) (`Timeline|PointLightTimeline` :!via `PlayFromStart`)
        (:`Update`
          (`LightComponent.SetIntensity` (`self.PointLight`) _intensitylight))))))

(fn `UserConstructionScript`)